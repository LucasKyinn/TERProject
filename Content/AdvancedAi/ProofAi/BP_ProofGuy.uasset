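; BP_ProofGuy is a proof-of-concept AI character for Q-learning, animated through a German Shepherd movement state.
; BeginPlay writes exploration epsilon to the blackboard, then loads and prints any saved state-action reward map from the MapProof slot.
; Tick fixes walk speed at the fast value and derives the movement state from crouch and speed bands.
; GetState encodes the nearest TargetPoint's rounded position and goal distance as a string key.
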(event `self.ReceiveTick`
  (params (DeltaSeconds :type "Float (single-precision)"))
  (bind _speed (`self.Speed`))
  (bind _charactermovement (`self.CharacterMovement`))
  (`|ExecutionSequence`
    (:`then_0`
      ;[1 1 1] Set Max WalkSpeed
      (if true
        (set `CharacterMovementComponent.MaxWalkSpeed` 1000.0 _charactermovement)
        (else
          (set `CharacterMovementComponent.MaxWalkSpeed` 550.0 _charactermovement))))
    (:`then_1`
      (set `self.Speed` (`KismetMathLibrary.VSize` (`self.GetVelocity`)))
      ;[1 1 1] Animation stuff
      (if (`self.Crouched`)
        (set `self.GermanShepardMovement` "NewEnumerator2")
        (elif (`KismetMathLibrary.NearlyEqual_FloatFloat` _speed 0.0 0.5)
          (set `self.GermanShepardMovement` "NewEnumerator8")
          (elif (and (> _speed 1.0) (<= _speed 300.0))
            (set `self.GermanShepardMovement` "NewEnumerator1")
            (elif (and (> _speed 300.0) (<= _speed 600.0))
              (set `self.GermanShepardMovement` "NewEnumerator0")
              (elif (and (> _speed 600.0) (<= _speed 900.0))
                (set `self.GermanShepardMovement` "NewEnumerator3")
                (elif (and (> _speed 900.0) (<= _speed 1100.0))
                  (set `self.GermanShepardMovement` "NewEnumerator4")
                  (elif (> _speed 1100.0)
                    (set `self.GermanShepardMovement` "NewEnumerator5")))))))))))

(event `self.ReceiveBeginPlay`
  ;[1 1 1] Save Action/Reward Map
  (`BlackboardComponent.SetValueAsFloat` (`AIBlueprintHelperLibrary.GetBlackboard` self) "Epsilon" 0.06)
  (bind _returnvalue (`GameplayStatics.DoesSaveGameExist` "MapProof"))
  (if _returnvalue
    (bind _returnvalue_2 (`GameplayStatics.LoadGameFromSlot` "MapProof"))
    (bind _asbp_save_map (cast `/Game/AdvancedAi/CoopAI/BP_SaveMap` _returnvalue_2))
    (bind _output_get (set `self.StateActionToQReward` (`/Game/AdvancedAi/CoopAI/BP_SaveMap.StateActionToQReward` _asbp_save_map)))
    ;[1 1 1] Print Loaded Map Content
    (bind _keys (`BlueprintMapLibrary.Map_Keys` _output_get))
    (bind _values (`BlueprintMapLibrary.Map_Values` _output_get))
    (for (_array_element _array_index) _keys
      (`KismetSystemLibrary.PrintString` (`KismetStringLibrary.Concat_StrStr` _array_element " : " (`KismetStringLibrary.Conv_DoubleToString` (`|GetArrayItem` _values _array_index)))))))

(fn `GetState`
  (returns (State :type String))
  (locals (Closest :type "TargetPoint Object Reference"))
  (bind _returnvalue (`self.K2_GetActorLocation` (`local.Closest`)))
  (bind (_x _y) (`KismetMathLibrary.BreakVector2D` (`KismetMathLibrary.Conv_VectorToVector2D` _returnvalue)))
  (bind _outactors (`GameplayStatics.GetAllActorsOfClass` "/Script/Engine.TargetPoint"))
  (set `local.Closest` (`|GetArrayItem` _outactors))
  (for (_array_element _array_index) _outactors
    (if (!= _array_index 0)
      (if (< (`self.GetDistanceTo` _array_element) (`self.GetDistanceTo` (`local.Closest`)))
        (set `local.Closest` _array_element))))
  (bind _returnvalue_2 (`GameplayStatics.GetActorOfClass` "/Game/AdvancedAi/ProofAi/TargetPointGoal.TargetPointGoal_C"))
  (return (`KismetStringLibrary.Concat_StrStr` (`KismetStringLibrary.Conv_IntToString` (`KismetMathLibrary.Round` _x)) ";" (`KismetStringLibrary.Conv_IntToString` (`KismetMathLibrary.Round` _y)) ";" (`KismetStringLibrary.Conv_IntToString` (`KismetMathLibrary.Round` (`KismetMathLibrary.Vector_Distance` _returnvalue (`self.K2_GetActorLocation` _returnvalue_2)))))))

(fn `UserConstructionScript`)