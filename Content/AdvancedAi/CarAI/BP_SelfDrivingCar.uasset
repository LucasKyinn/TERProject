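; Early-stage self-driving car actor that so far only senses what is ahead and does not drive.
; Each Tick it sphere-traces on the Visibility channel from the front bumper along its horizontal forward direction, with debug drawing.
; The trace result is unused, and a node that would nudge the actor forward is never executed.
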(event `self.ReceiveTick`
  (params (DeltaSeconds :type "Float (single-precision)"))
  (bind _frontbumperforward (`self.FrontBumperForward`))
  (bind _returnvalue (`SceneComponent.K2_GetComponentLocation` _frontbumperforward))
  (`KismetSystemLibrary.SphereTraceSingle` :`Start` _returnvalue :`End` (+ _returnvalue (* (`SceneComponent.GetForwardVector` _frontbumperforward) (2000.0 2000.0 0.0))) :`Radius` 15.0 :`TraceChannel` "TraceTypeQuery1" :`DrawDebugType` "ForDuration" :`DrawTime` 0.0))

(fn `UserConstructionScript`)