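; AI controller for the co-op German Shepard dog, which starts the BT_Shepard behavior tree on BeginPlay.
; It also holds an unconnected epsilon-greedy Q-learning experiment that sets a blackboard Action, reads pawn state and stores Q-values in a state-action map.
; NewQ implements the standard Q-update, but the reward and max-future-Q helpers are stubs returning zero, so none of the learning is active.
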(event `self.ReceiveBeginPlay`
  (`self.RunBehaviorTree` "/Game/AdvancedAi/CoopAI/BT_Shepard.BT_Shepard"))

(fn `CaluclateReward`
  (params (State :type String) (NewState :type String))
  (returns (Reward :type Integer))
  (return 0))

(fn `Find Max Futur Q`
  (params (Map :type "Map of String to Float (double-precision)"))
  (returns (MaxFutureQ :type "Float (double-precision)"))
  (return 0.0))

(fn `New Q`
  (params (CurrentQ :type "Float (double-precision)") (MaxFutureQ :type "Float (double-precision)") (Alpha :type "Float (double-precision)") (Gamma :type "Float (double-precision)") (Reward :type Integer))
  (returns (NewQ :type "Float (double-precision)"))
  (return (+ (* (- 1.0 Alpha) CurrentQ) (* Alpha (+ (* Gamma MaxFutureQ) (`KismetMathLibrary.Conv_IntToDouble` Reward))))))

(fn `UserConstructionScript`)