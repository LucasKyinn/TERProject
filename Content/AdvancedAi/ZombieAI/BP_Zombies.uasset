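; BP_Zombies is an AI zombie with pawn sensing that tracks a target and reacts to noise.
; Each tick it draws a debug sphere around itself and, until dead, copies the blackboard's TargetActor into Targeting.
; On hearing noise, it checks InCombat, a comparison on Targeting, and if true sets its yaw directly to the noise location's X coordinate rather than a computed look-at angle.
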(event `self.ReceiveTick`
  (params (DeltaSeconds :type "Float (single-precision)"))
  (`KismetSystemLibrary.DrawDebugSphere` (`self.K2_GetActorLocation`) 1500.0)
  (if (not (`self.bDied`))
    (set `self.Targeting` (`BlackboardComponent.GetValueAsObject` (`AIBlueprintHelperLibrary.GetBlackboard` null) "TargetActor"))))

(event `self.PawnSensingComp.OnHearNoise`
  (params (Instigator :type "Pawn Object Reference") (Location :type "Vector Structure (by ref)") (Volume :type "Float (single-precision)"))
  (bind _return (`self.InCombat`))
  (if _return
    (`self.K2_SetActorRotation` (`KismetMathLibrary.MakeRotator` 0.0 0.0 (.x Location)))))

(fn `InCombat`
  (returns (Return :type Boolean))
  (bind _returnvalue (== (`self.Targeting`) null))
  (if _returnvalue
    (return _returnvalue)))

(fn `UserConstructionScript`)